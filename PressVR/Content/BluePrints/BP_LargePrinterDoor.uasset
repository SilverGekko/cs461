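; Large printer door actor that toggles between open and closed rotations on touch enter or motion controller pickup.
; BeginPlay runs the same toggle, and Drop does nothing.
; Each toggle applies a single RInterpTo step toward the target rotation, with no tick or timeline continuing it, then flips IsOpen.
; The opening branch also sets T11 to 4 on the first LevelDatabaseActor found.
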(event EventBeginPlay
  (if (Variables|Default|GetIsOpen)
    (Transformation|SetActorRotation (Math|Interpolation|RInterpTo (Transformation|GetActorRotation) (Variables|Default|GetClosedRotation) (Variables|Default|GetDeltaTimeSeconds) (Variables|Default|GetRotSpeed)))
    (Variables|Default|SetIsOpen false)
    (else
      (Transformation|SetActorRotation (Math|Interpolation|RInterpTo (Transformation|GetActorRotation) (Variables|Default|GetOpenRotation) (Variables|Default|GetDeltaTimeSeconds) (Variables|Default|GetRotSpeed)))
      (Variables|Default|SetIsOpen true)
      (bind _outactors (Actor|GetAllActorsOfClass "/Game/BluePrints/LevelDatabaseActor.LevelDatabaseActor_C"))
      (Variables|/Game/BluePrints/LevelDatabaseActor.LevelDatabaseActor_C|SetT_1_1 (Utilities|Array|Get(acopy) _outactors) 4))))

(event EventActorOnInputTouchEnter
  (params (FingerIndex :type ETouchIndex%20Enum :default "Touch1"))
  (if (Variables|Default|GetIsOpen)
    (Transformation|SetActorRotation (Math|Interpolation|RInterpTo (Transformation|GetActorRotation) (Variables|Default|GetClosedRotation) (Variables|Default|GetDeltaTimeSeconds) (Variables|Default|GetRotSpeed)))
    (Variables|Default|SetIsOpen false)
    (else
      (Transformation|SetActorRotation (Math|Interpolation|RInterpTo (Transformation|GetActorRotation) (Variables|Default|GetOpenRotation) (Variables|Default|GetDeltaTimeSeconds) (Variables|Default|GetRotSpeed)))
      (Variables|Default|SetIsOpen true)
      (bind _outactors (Actor|GetAllActorsOfClass "/Game/BluePrints/LevelDatabaseActor.LevelDatabaseActor_C"))
      (Variables|/Game/BluePrints/LevelDatabaseActor.LevelDatabaseActor_C|SetT_1_1 (Utilities|Array|Get(acopy) _outactors) 4))))

(event EventPickup
  (params (AttachTo :type Scene%20Component%20Object%20Reference))
  (if (Variables|Default|GetIsOpen)
    (Transformation|SetActorRotation (Math|Interpolation|RInterpTo (Transformation|GetActorRotation) (Variables|Default|GetClosedRotation) (Variables|Default|GetDeltaTimeSeconds) (Variables|Default|GetRotSpeed)))
    (Variables|Default|SetIsOpen false)
    (else
      (Transformation|SetActorRotation (Math|Interpolation|RInterpTo (Transformation|GetActorRotation) (Variables|Default|GetOpenRotation) (Variables|Default|GetDeltaTimeSeconds) (Variables|Default|GetRotSpeed)))
      (Variables|Default|SetIsOpen true)
      (bind _outactors (Actor|GetAllActorsOfClass "/Game/BluePrints/LevelDatabaseActor.LevelDatabaseActor_C"))
      (Variables|/Game/BluePrints/LevelDatabaseActor.LevelDatabaseActor_C|SetT_1_1 (Utilities|Array|Get(acopy) _outactors) 4))))

(event EventDrop)

(fn ConstructionScript)