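; BP_SidedoorLow is the lower half of a side door that toggles between open and closed on touch or motion-controller pickup.
; BeginPlay, touch enter and Pickup share one toggle that flips IsOpen and also rotates the linked HighDoor actor.
; This door takes a single RInterpTo step per trigger, with no tick or timeline, while HighDoor snaps straight to its target rotation.
; Drop does nothing.
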(event EventBeginPlay
  (if (Variables|Default|GetIsOpen)
    (Transformation|SetActorRotation (Math|Interpolation|RInterpTo (Transformation|GetActorRotation) (Variables|Default|GetClosedRotation) (Variables|Default|GetDeltaTimeSeconds) (Variables|Default|GetRotSpeed)))
    (Variables|Default|SetIsOpen false)
    (Transformation|SetActorRotation (Variables|Default|GetHighDoor) (Variables|Default|GetClosedRotation) true)
    (else
      (Transformation|SetActorRotation (Math|Interpolation|RInterpTo (Transformation|GetActorRotation) (Variables|Default|GetOpenRotation) (Variables|Default|GetDeltaTimeSeconds) (Variables|Default|GetRotSpeed)))
      (Variables|Default|SetIsOpen true)
      (Transformation|SetActorRotation (Variables|Default|GetHighDoor) (Variables|Default|GetHighDoorOpenRot)))))

(event EventActorOnInputTouchEnter
  (params (FingerIndex :type ETouchIndex%20Enum :default "Touch1"))
  (if (Variables|Default|GetIsOpen)
    (Transformation|SetActorRotation (Math|Interpolation|RInterpTo (Transformation|GetActorRotation) (Variables|Default|GetClosedRotation) (Variables|Default|GetDeltaTimeSeconds) (Variables|Default|GetRotSpeed)))
    (Variables|Default|SetIsOpen false)
    (Transformation|SetActorRotation (Variables|Default|GetHighDoor) (Variables|Default|GetClosedRotation) true)
    (else
      (Transformation|SetActorRotation (Math|Interpolation|RInterpTo (Transformation|GetActorRotation) (Variables|Default|GetOpenRotation) (Variables|Default|GetDeltaTimeSeconds) (Variables|Default|GetRotSpeed)))
      (Variables|Default|SetIsOpen true)
      (Transformation|SetActorRotation (Variables|Default|GetHighDoor) (Variables|Default|GetHighDoorOpenRot)))))

(event EventPickup
  (params (AttachTo :type Scene%20Component%20Object%20Reference))
  (if (Variables|Default|GetIsOpen)
    (Transformation|SetActorRotation (Math|Interpolation|RInterpTo (Transformation|GetActorRotation) (Variables|Default|GetClosedRotation) (Variables|Default|GetDeltaTimeSeconds) (Variables|Default|GetRotSpeed)))
    (Variables|Default|SetIsOpen false)
    (Transformation|SetActorRotation (Variables|Default|GetHighDoor) (Variables|Default|GetClosedRotation) true)
    (else
      (Transformation|SetActorRotation (Math|Interpolation|RInterpTo (Transformation|GetActorRotation) (Variables|Default|GetOpenRotation) (Variables|Default|GetDeltaTimeSeconds) (Variables|Default|GetRotSpeed)))
      (Variables|Default|SetIsOpen true)
      (Transformation|SetActorRotation (Variables|Default|GetHighDoor) (Variables|Default|GetHighDoorOpenRot)))))

(event EventDrop)

(fn ConstructionScript)