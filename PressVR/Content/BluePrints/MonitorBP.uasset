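; Monitor Blueprint whose plane screen blinks between a Webpress UI and its error variant until stage completion.
; Every Tick it looks up the first LevelDatabaseActor and reads S1StageXComplete to either blink or hold the normal screen.
; The textureBlinking graph alternates on TextureSwitch with unequal Delays, showing the error screen longer.
; It creates a dynamic material instance before each SetMaterial, which then applies the plain material instead.
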(event EventTick
  (params (DeltaSeconds :type Float%20%28single-precision%29))
  (bind _outactors (Actor|GetAllActorsOfClass "/Game/BluePrints/LevelDatabaseActor.LevelDatabaseActor_C"))
  (if (Variables|/Game/BluePrints/LevelDatabaseActor.LevelDatabaseActor_C|GetS1_StageX_Complete (Utilities|Array|Get(acopy) _outactors))
    (goto _label execute2)
    (else
      (|textureBlinking :!label _label))))

(fn ConstructionScript)