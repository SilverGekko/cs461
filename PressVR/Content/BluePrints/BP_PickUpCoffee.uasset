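; BP_PickUpCoffee is a coffee pickup actor that BP_MotionController can grab and release.
; Pickup flags ObjectGrabed on the first LevelDatabaseActor, turns off mesh physics and attaches the root to the given component, keeping its world transform.
; Drop re-enables physics and detaches the actor, leaving the ObjectGrabed flag untouched.
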(event EventPickup
  (params (AttachTo :type Scene%20Component%20Object%20Reference))
  (bind _outactors (Actor|GetAllActorsOfClass "/Game/BluePrints/LevelDatabaseActor.LevelDatabaseActor_C"))
  (Variables|/Game/BluePrints/LevelDatabaseActor.LevelDatabaseActor_C|SetObjectGrabed (Utilities|Array|Get(acopy) _outactors) true)
  (Physics|SetSimulatePhysics (Variables|Debug|GetStaticMeshComponent) false)
  (Transformation|AttachComponentToComponent (VehicleSound|GetRootComponent) AttachTo "None" "KeepWorld" "KeepWorld" "KeepWorld" false))

(event EventDrop
  (Physics|SetSimulatePhysics (Variables|Debug|GetStaticMeshComponent) true)
  (Transformation|DetachFromActor "KeepWorld" "KeepWorld" "KeepWorld"))

(fn ConstructionScript)